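; Ore piece actor that shows a red, green or cyan sprite and responds to mouse clicks or touches.
; SetOreType stores the type and swaps the sprite, starting from type 0 on BeginPlay.
; SetOreStatus stores the state, enlarging the sprite when chosen and toggling its visibility when pending delete.
; Clicks and touches on the sprite both call OrePress with a finger index.
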(event `self.ReceiveBeginPlay`
  (`self.SetOreType` 0))

(event `self.ReceiveActorBeginOverlap`
  (params (OtherActor :type "Actor Object Reference")))

(event `self.ReceiveTick`
  (params (DeltaSeconds :type "Float (single-precision)")))

(event `self.OreSprite.OnClicked`
  (params (TouchedComponent :type "PrimitiveComponent Object Reference") (ButtonPressed :type "Key Structure"))
  (`self.OrePress` (stale `self.OreSprite.OnInputTouchBegin` FingerIndex) :!label _label))

(event `self.OreSprite.OnInputTouchBegin`
  (params (FingerIndex :type "ETouchIndex Enum" :default "Touch1") (TouchedComponent :type "PrimitiveComponent Object Reference"))
  (goto _label))

(fn `SetOreStatus`
  (params (NewStatus :type Integer))
  (bind _oresprite (`self.OreSprite`))
  (switch `EOreStatus` (cast `EOreStatus` (`KismetMathLibrary.Conv_IntToByte` NewStatus))
    (:`EOS_Normal`
      (`SceneComponent.SetVisibility` _oresprite true false)
      (`SceneComponent.SetRelativeScale3D` _oresprite (2.0 2.0 2.0) :!label _label))
    (:`EOS_Moving`
      (goto _label))
    (:`EOS_Choosen`
      (`SceneComponent.SetRelativeScale3D` _oresprite (3.0 3.0 3.0)))
    (:`EOS_PendingDelete`
      (`SceneComponent.ToggleVisibility` _oresprite false)
      (goto _label)))
  (set `self.OreStatus` NewStatus))

(fn `SetOreType`
  (params (NewType :type Integer))
  (bind _oresprite (`self.OreSprite`))
  (set `self.OreType` NewType)
  (switch `EOreType` (cast `EOreType` (`KismetMathLibrary.Conv_IntToByte` NewType))
    (:`EOT_Red`
      (`PaperSpriteComponent.SetSprite` _oresprite "/Game/Sprites/Red_Ore_Sprite.Red_Ore_Sprite"))
    (:`EOT_Green`
      (`PaperSpriteComponent.SetSprite` _oresprite "/Game/Sprites/Green_Ore_Sprite.Green_Ore_Sprite"))
    (:`EOT_Cyan`
      (`PaperSpriteComponent.SetSprite` _oresprite "/Game/Sprites/Cyan_Ore_Sprite.Cyan_Ore_Sprite"))))

(fn `UserConstructionScript`)